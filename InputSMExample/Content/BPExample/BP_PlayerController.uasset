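; Example player controller that turns keyboard presses into gamepad-style input for an input state machine.
; Q, W, E, A, D, Z, X and C presses set button and trigger flags in InputFrame; this graph never clears them.
; Tick passes the frame to InputSM, which runs from BeginPlay to EndPlay, and prints the active state name when processing returns true.
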(event `InputAction|Q`
  (params (Key :type "Key Structure"))
  (:`Pressed`
    (setmembers `InputFrame` :`StructRef` (`self.InputFrame`) :`LeftUpperTrigger` true)))

(event `InputAction|W`
  (params (Key :type "Key Structure"))
  (:`Pressed`
    (setmembers `InputFrame` :`StructRef` (`self.InputFrame`) :`B` true)))

(event `InputAction|E`
  (params (Key :type "Key Structure"))
  (:`Pressed`
    (setmembers `InputFrame` :`StructRef` (`self.InputFrame`) :`RightUpperTrigger` true)))

(event `InputAction|A`
  (params (Key :type "Key Structure"))
  (:`Pressed`
    (setmembers `InputFrame` :`StructRef` (`self.InputFrame`) :`A` true)))

(event `InputAction|D`
  (params (Key :type "Key Structure"))
  (:`Pressed`
    (setmembers `InputFrame` :`StructRef` (`self.InputFrame`) :`Y` true)))

(event `InputAction|Z`
  (params (Key :type "Key Structure"))
  (:`Pressed`
    (setmembers `InputFrame` :`StructRef` (`self.InputFrame`) :`LeftTrigger` true)))

(event `InputAction|X`
  (params (Key :type "Key Structure"))
  (:`Pressed`
    (setmembers `InputFrame` :`StructRef` (`self.InputFrame`) :`X` true)))

(event `InputAction|C`
  (params (Key :type "Key Structure"))
  (:`Pressed`
    (setmembers `InputFrame` :`StructRef` (`self.InputFrame`) :`RightTrigger` true)))

(event `self.ReceiveTick`
  (params (DeltaSeconds :type "Float (single-precision)"))
  (bind _inputsm (`self.InputSM`))
  (bind _states (`InputSM.States` _inputsm))
  (bind _activestateindex (`InputSM.ActiveStateIndex` _inputsm))
  (bind _output_statename (break `InputSM_State` (`|GetArrayItem` _states _activestateindex)))
  (`/Engine/EditorBlueprintResources/StandardMacros.IsValid` _inputsm
    (:`Is Valid`
      (bind _returnvalue (`InputSM.ProcessInput` _inputsm (`self.InputFrame`)))
      (if _returnvalue
        (if (`KismetArrayLibrary.Array_IsValidIndex` _states _activestateindex)
          (`KismetSystemLibrary.PrintString` (`KismetStringLibrary.Conv_NameToString` _output_statename)))))))

(event `self.ReceiveBeginPlay`
  (`InputSM.Start` (`self.InputSM`)))

(event `self.ReceiveEndPlay`
  (params (EndPlayReason :type "EEndPlayReason Enum" :default "Destroyed"))
  (`InputSM.Stop` (`self.InputSM`)))

(fn `UserConstructionScript`)